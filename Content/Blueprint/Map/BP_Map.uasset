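; BP_Map generates a procedural hex map of BP_CitySlot actors and handles slot selection on it.
; One Perlin noise cuts out ocean gaps, while another sets each tile's height and color band, with random yellow tiles on low coasts.
; SelectSlot moves a lazily created selector mesh, then DistanceCalcul recolors every slot and stores its cube-coordinate hex distance from that point.
; DeleteMap destroys all slots.
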(event `GenerateNoise`
  (bind _returnvalue (`|GenericCreateObject` "/Script/FastNoiseGenerator.FastNoiseWrapper"))
  (`FastNoiseWrapper.SetupFastNoise` _returnvalue "Perlin" 1337 0.1 "Quintic" "FBM" 3 2.0 0.5 0.45 "Euclidean" "CellValue")
  (set `self.FastNoise` _returnvalue)
  (bind _returnvalue_2 (`|GenericCreateObject` "/Script/FastNoiseGenerator.FastNoiseWrapper"))
  (`FastNoiseWrapper.SetupFastNoise` _returnvalue_2 "Perlin" 1995 0.15 "Quintic" "FBM" 3 3.0 0.5 0.45 "Manhattan" "CellValue")
  (set `self.FastnoiseOcean` _returnvalue_2))

(event `BuildMap`
  (bind _returnvalue (/ (`self.GridY`) 2))
  (bind _returnvalue_2 (/ (`self.GridX`) 2))
  ;[0.3757 0.7325 1] Build Map
  (for _index (range (* _returnvalue_2 -1) (+ _returnvalue_2 1))
    (for _index_2 (range (* _returnvalue -1) (+ _returnvalue 1))
      (bind _returnvalue_3 (`FastNoiseWrapper.GetNoise2D` (`self.FastnoiseOcean`) (`KismetMathLibrary.Conv_IntToDouble` _index) (`KismetMathLibrary.Conv_IntToDouble` _index_2)))
      (if (not (< _returnvalue_3 -0.1))
        (bind _returnvalue_4 (`KismetMathLibrary.Conv_IntToDouble` _index_2))
        (bind _returnvalue_5 (`KismetMathLibrary.Conv_IntToDouble` _index))
        (bind _returnvalue_6 (* _returnvalue_5 100.0))
        (bind _returnvalue_7 (`|SpawnActorFromClass` "/Game/Blueprint/Map/BP_CitySlot.BP_CitySlot_C" (`KismetMathLibrary.MakeTransform` (`KismetMathLibrary.MakeVector` (* _returnvalue_4 100.0) (`KismetMathLibrary.SelectFloat` _returnvalue_6 (+ _returnvalue_6 50.0) (`/Game/Blueprint/BFL_Utility.IsOdd` _index_2))) (struct :`Yaw` 90.0) (0.5 0.5 0.5)) "Undefined" "OverrideRootScale" null null))
        (bind _staticmesh (`/Game/Blueprint/Map/BP_CitySlot.StaticMesh` _returnvalue_7))
        (bind _returnvalue_8 (`KismetMathLibrary.FClamp` (`FastNoiseWrapper.GetNoise2D` (`self.FastNoise`) _returnvalue_5 _returnvalue_4)))
        (`SceneComponent.K2_SetRelativeLocation` _staticmesh (`KismetMathLibrary.MakeVector` 0.0 0.0 (* _returnvalue_8 400.0)) false false)
        (bind _returnvalue_9 (`KismetMathLibrary.FTrunc` (`KismetMathLibrary.FClamp` (* _returnvalue_8 20.0) 0.0 10.0)))
        (if (and (`KismetMathLibrary.RandomBoolWithWeight` 0.66) (< _returnvalue_3 0.0) (== _returnvalue_9 0))
          (`MeshComponent.SetVectorParameterValueOnMaterials` _staticmesh "Color" (1.0 1.0 0.0))
          (`MeshComponent.SetVectorParameterValueOnMaterials` _staticmesh "Gamma" (1.0 1.0 0.0))
          (else
            (`self.HeightColor` _staticmesh _returnvalue_9)))))))

(event `DeleteMap`
  ;[1 0.4158 0.4457] Delete Map
  (bind _outactors (`GameplayStatics.GetAllActorsOfClass` "/Game/Blueprint/Map/BP_CitySlot.BP_CitySlot_C"))
  (for _array_element _outactors
    (`self.K2_DestroyActor` _array_element)))

(event `SelectSlot`
  (params (Location :type "Vector Structure"))
  ;[0.5966 1 0.4339] Select on the Map
  (`|ExecutionSequence`
    (:`then_0`
      (`/Engine/EditorBlueprintResources/StandardMacros.DoOnce` false
        (:`Completed`
          (bind _returnvalue (`AddComponent|NODE_AddStaticMeshComponent-0`))
          (`StaticMeshComponent.SetStaticMesh` _returnvalue "/Game/StaticMesh/MapMesh/Hexa_Base_044.Hexa_Base_044")
          (`SceneComponent.SetWorldScale3D` _returnvalue (0.5 0.5 0.5))
          (`SceneComponent.K2_SetWorldRotation` _returnvalue (struct :`Yaw` 90.0) false false)
          (set `self.SelectorMesh` _returnvalue))))
    (:`then_1`
      (`SceneComponent.K2_SetWorldLocation` (`self.SelectorMesh`) Location false false)
      (set `self.Location` Location)
      (`self.DistanceCalcul`))))

(fn `DistanceCalcul`
  (bind (_location_x _location_y) (`KismetMathLibrary.BreakVector` (`self.Location`)))
  (bind _returnvalue (/ _location_x 100.0))
  (bind _returnvalue_2 (- (/ _location_y 100.0) (/ _returnvalue 2.0)))
  (bind _outactors (`GameplayStatics.GetAllActorsOfClass` "/Game/Blueprint/Map/BP_CitySlot.BP_CitySlot_C"))
  (for _array_element _outactors
    (bind (_returnvalue_x _returnvalue_y) (`KismetMathLibrary.BreakVector` (`SceneComponent.K2_GetComponentLocation` (`/Game/Blueprint/Map/BP_CitySlot.StaticMesh` _array_element))))
    (bind _returnvalue_3 (/ _returnvalue_x 100.0))
    (bind _returnvalue_4 (- (/ _returnvalue_y 100.0) (/ _returnvalue_3 2.0)))
    (bind _returnvalue_5 (/ (+ (`KismetMathLibrary.Abs` (- _returnvalue_3 _returnvalue)) (`KismetMathLibrary.Abs` (- (+ _returnvalue_3 _returnvalue_4) _returnvalue _returnvalue_2)) (`KismetMathLibrary.Abs` (- _returnvalue_4 _returnvalue_2))) 2.0))
    (`/Game/Blueprint/Map/BP_CitySlot.ChangeColor` _array_element (`KismetMathLibrary.FTrunc` _returnvalue_5))
    (set `/Game/Blueprint/Map/BP_CitySlot.DistanceFromCenter` _returnvalue_5 _array_element)))

(fn `HeightColor`
  (params (Target :type "MeshComponent Object Reference") (Height :type Integer))
  (`MeshComponent.SetVectorParameterValueOnMaterials` Target "Color" (select `/Game/Blueprint/Enum_Colors` (select `int` Height :`0` "NewEnumerator0" :`1` "NewEnumerator1" :`2` "NewEnumerator2" :`3` "NewEnumerator3" :`4` "NewEnumerator4" :`5` "NewEnumerator5" :`6` "NewEnumerator6" :`7` "NewEnumerator7" :`8` "NewEnumerator8" :`9` "NewEnumerator9" :`10` "NewEnumerator10" :`11` "NewEnumerator11" :`12` "NewEnumerator12" :`13` "NewEnumerator13" :`14` "NewEnumerator14" :`15` "NewEnumerator15" :`16` "NewEnumerator16" :`17` "NewEnumerator17" :`18` "NewEnumerator18" :`19` "NewEnumerator19" :`20` "NewEnumerator20" :`21` "NewEnumerator21" :`22` "NewEnumerator22" :!type "/Game/Blueprint/Enum_Colors Enum") :`NewEnumerator0` (0.0 1.0 0.0) :`NewEnumerator1` (0.0 1.0 0.25) :`NewEnumerator2` (0.0 1.0 0.5) :`NewEnumerator3` (0.25 0.15 0.01) :`NewEnumerator4` (0.25 0.15 0.01) :`NewEnumerator5` (0.5 0.5 0.5) :`NewEnumerator6` (0.5 0.5 0.5) :`NewEnumerator7` (0.5 0.5 0.5) :`NewEnumerator8` (0.6 0.6 0.6) :`NewEnumerator9` (1.0 1.0 1.0) :`NewEnumerator10` (2.0 2.0 2.0) :`NewEnumerator11` (3.0 3.0 3.0) :`NewEnumerator12` (1.0 1.0 1.0) :`NewEnumerator13` (1.0 1.0 1.0) :`NewEnumerator14` (1.0 1.0 1.0) :`NewEnumerator15` (1.0 1.0 1.0) :`NewEnumerator16` (1.0 1.0 1.0) :`NewEnumerator17` (1.0 1.0 1.0) :`NewEnumerator18` (1.0 1.0 1.0) :`NewEnumerator19` (1.0 1.0 1.0) :`NewEnumerator20` (1.0 1.0 1.0) :`NewEnumerator21` (1.0 1.0 1.0) :`NewEnumerator22` (1.0 1.0 1.0) :!type "Vector Structure"))
  (if (== Height 10)
    (`MeshComponent.SetVectorParameterValueOnMaterials` Target "Gamma" (1.0 1.0 1.0))))

(fn `UserConstructionScript`)