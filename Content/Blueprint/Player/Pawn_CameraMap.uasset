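; Camera pawn for the map, handling zoom, rotation, panning and slot selection through its spring arm.
; Zoom changes the clamped arm length, while rotate and grab inputs run looping timers that yaw or move the arm.
; Tick measures grab hold time to tell a drag from a short click, which traces under the cursor and calls SelectSlot on BP_Map.
; The W key prints the hovered city slot's distance from center.
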(event `InputAxis|InputAxisZoom`
  (params (AxisValue :type "Float (single-precision)"))
  (bind _springarm (`self.SpringArm`))
  ;[1 0.5773 0.1936] Zoom/DeZoom on the Map
  (set `SpringArmComponent.TargetArmLength` (`KismetMathLibrary.FClamp` (+ (`SpringArmComponent.TargetArmLength` _springarm) (* AxisValue 100.0)) 800.0 2400.0) _springarm))

(event `InputAction|InputActionRotate`
  (params (Key :type "Key Structure"))
  ;[0.7552 1 0.2705] Rotate along Z on the Map
  (:`Pressed`
    (bind _returnvalue (`KismetSystemLibrary.K2_SetTimerDelegate` (delegate `UpdateRotation`) 0.005 true))
    (set `self.handlerRotateTimer` _returnvalue))
  (:`Released`
    (`KismetSystemLibrary.K2_ClearAndInvalidateTimerHandle` (`self.handlerRotateTimer`))))

(event `UpdateRotation`
  ;[0.7552 1 0.2705] Rotate along Z on the Map
  (`SceneComponent.K2_AddRelativeRotation` (`self.SpringArm`) (`KismetMathLibrary.MakeRotator` 0.0 0.0 (* (`self.GetInputAxisValue`) 0.2 -1.0)) false false))

(event `InputAction|InputActionGrab`
  (params (Key :type "Key Structure"))
  (bind (_hitresult _returnvalue) (`PlayerController.GetHitResultUnderCursorByChannel` (`GameplayStatics.GetPlayerController` 0) "TraceTypeQuery1" true))
  ;[0.7552 1 0.2705] Move along X and Y on the Map
  (:`Pressed`
    (set `self.Click?` true))
  (:`Released`
    (set `self.Click?` false)
    (if (< (`self.TimeHolded`) 0.25)
      (if _returnvalue
        (bind _returnvalue_2 (`GameplayStatics.GetActorOfClass` "/Game/Blueprint/Map/BP_Map.BP_Map_C"))
        (`/Game/Blueprint/Map/BP_Map.SelectSlot` _returnvalue_2 (`KismetMathLibrary.MakeVector` (.x (`SceneComponent.K2_GetComponentLocation` (`.HitComponent` (`GameplayStatics.BreakHitResult` _hitresult)))) (.y (`SceneComponent.K2_GetComponentLocation` (`.HitComponent` (`GameplayStatics.BreakHitResult` _hitresult)))) (+ (.z (`SceneComponent.K2_GetComponentLocation` (`.HitComponent` (`GameplayStatics.BreakHitResult` _hitresult)))) 1.0))))
      (set `self.TimeHolded` 0.0)
      (goto _label :!via `Reset`)
      (else
        (set `self.TimeHolded` 0.0)
        (`KismetSystemLibrary.K2_ClearAndInvalidateTimerHandle` (`self.HandlerGrabTimer`))
        (goto _label :!via `Reset`)))))

(event `self.ReceiveTick`
  (params (DeltaSeconds :type "Float (single-precision)"))
  (bind _timeholded (`self.TimeHolded`))
  ;[1 0.8422 0.1435] Click or Hold
  (if (`self.Click?`)
    (set `self.TimeHolded` (+ _timeholded DeltaSeconds))
    (if (> _timeholded 0.25)
      (`/Engine/EditorBlueprintResources/StandardMacros.DoOnce` false :!label _label
        (:`Completed`
          (bind _returnvalue (`KismetSystemLibrary.K2_SetTimerDelegate` (delegate `UpdateGrab`) 0.005 true))
          (set `self.HandlerGrabTimer` _returnvalue))))))

(event `UpdateGrab`
  ;[1 0.8422 0.1435] Click or Hold
  (`SceneComponent.K2_AddRelativeLocation` (`self.SpringArm`) (`KismetMathLibrary.MakeVector` (`self.GetInputAxisValue`) (`self.GetInputAxisValue`)) false false))

(event `Key|W`
  (params (Key :type "Key Structure"))
  (:`Pressed`
    (bind _asbp_city_slot (cast `/Game/Blueprint/Map/BP_CitySlot` (`.HitActor` (`GameplayStatics.BreakHitResult` (`PlayerController.GetHitResultUnderCursorByChannel` (`GameplayStatics.GetPlayerController` 0) "TraceTypeQuery1" true)))))
    (`KismetSystemLibrary.PrintString` (`KismetStringLibrary.Conv_DoubleToString` (`/Game/Blueprint/Map/BP_CitySlot.DistanceFromCenter` _asbp_city_slot)))))

(fn `UserConstructionScript`)